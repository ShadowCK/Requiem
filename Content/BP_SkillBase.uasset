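; Base class for a leveled skill that a Caster casts using mana, with a cooldown between uses.
; Cast checks level, mana and cooldown, pays the cost, starts the cooldown and calls the empty OnCast hook for subclasses.
; Passive counts the cooldown down by delta time and calls the OnPassive hook.
; LevelUp spends a Caster skill point up to MaxLevel, and GetStat provides linear per-level scaling.
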(fn LevelUp
  (if (and (CallFunction|CanLevelUp) (Default|HasSkillPoint (Variables|Default|GetCaster)))
    (Math|Integer|IncrementInt (Variables|Default|GetLevel)
      (:%20%20
        (Math|Integer|DecrementInt (Variables|/Game/AC_Caster.AC_Caster_C|GetSkillPoints (Variables|Default|GetCaster)))))))

(fn Cast
  (if (CallFunction|CanCast)
    (Default|AddMana (Variables|Default|GetCaster) (* (Variables|Default|GetMana) -1.0))
    (Variables|Default|SetCooldownLeft (Variables|Default|GetCooldown))
    (CallFunction|OnCast (Variables|Default|GetLevel))
    (return true)
    (else
      (return false))))

(fn Passive
  (params (DeltaSeconds :type Float%20%28double-precision%29))
  (Variables|Default|SetCooldownLeft (- (Variables|Default|GetCooldownLeft) DeltaSeconds))
  (CallFunction|OnPassive DeltaSeconds))

(fn OnPassive
  (params (DeltaSeconds :type Float%20%28double-precision%29)))

(fn OnCast
  (params (Level :type Integer)))

(fn CanCast
  (return (and (not (or (CallFunction|IsNoMana) (CallFunction|IsonCooldown))) (> (Variables|Default|GetLevel) 0))))

(fn IsonCooldown
  (return (> (Variables|Default|GetCooldownLeft) 0.0)))

(fn IsNoMana
  (return (< (Variables|/Game/AC_Caster.AC_Caster_C|GetMana (Variables|Default|GetCaster)) (Variables|Default|GetMana))))

(fn CanLevelUp
  (return (< (Variables|Default|GetLevel) (Variables|Default|GetMaxLevel))))

(fn GetStat
  (params (Level :type Integer) (Base :type Float%20%28double-precision%29) (Scale :type Float%20%28double-precision%29))
  (return (+ Base (* Scale (- Level 1)))))