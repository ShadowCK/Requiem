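; AC_Caster is a component for the player that tracks mana, skill points and regeneration.
; BeginPlay casts the owner to BP_Player and stores it, and Tick applies health and mana regen scaled by delta time.
; Health is written to the player's CurrentHP while mana lives on the component, both clamped between zero and their maximum.
; A helper function reports whether any skill points remain.
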(event EventBeginPlay
  (bind _asbp_player (Utilities|Casting|CastToBP_Player (Components|GetOwner)))
  (Variables|Default|SetPlayer _asbp_player))

(event EventTick
  (params (DeltaSeconds :type Float%20%28single-precision%29))
  (CallFunction|Regen DeltaSeconds (Variables|Default|GetHealthRegen) (Variables|Default|GetManaRegen)))

(fn HasSkillPoint
  (return (> (Variables|Default|GetSkillPoints) 0)))

(fn AddHealth
  (params (Value :type Float%20%28double-precision%29))
  (bind _player (Variables|Default|GetPlayer))
  (Variables|/Game/Variant_Shooter/Blueprints/BP_ShooterCharacter.BP_ShooterCharacter_C|SetCurrent%20HP (Variables|Default|GetPlayer) (Math|Float|Max(Float) (Math|Float|Min(Float) (Variables|/Game/Variant_Shooter/Blueprints/BP_ShooterCharacter.BP_ShooterCharacter_C|GetMax%20HP _player) (+ Value (Variables|/Game/Variant_Shooter/Blueprints/BP_ShooterCharacter.BP_ShooterCharacter_C|GetCurrent%20HP _player))) 0.0)))

(fn AddMana
  (params (Value :type Float%20%28double-precision%29))
  (Variables|Default|SetMana (Math|Float|Max(Float) (Math|Float|Min(Float) (Variables|Default|GetMaxMana) (+ Value (Variables|Default|GetMana))) 0.0)))

(fn Regen
  (params (DeltaSeconds :type Float%20%28double-precision%29) (HeathRegen :type Float%20%28double-precision%29) (ManaRegen :type Float%20%28double-precision%29))
  (CallFunction|AddHealth (* DeltaSeconds HeathRegen))
  (CallFunction|AddMana (* DeltaSeconds ManaRegen)))