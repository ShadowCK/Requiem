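; Requiem shooter weapon that builds a clamped soul count and can fire homing soul projectiles.
; Each bullet fired adds a soul on top of the parent behavior.
; FireSoul spawns a randomly rotated soul projectile at the owning pawn, passing it a target and multiplied damage.
; OnRequiem clears CanGetSoul and starts a timer, with a separate function to restore the flag, which soul gain here never checks.
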(event EventBeginPlay
  (|CallParentFunction) ; This node is disabled and will not be called.\nDrag off pins to build functionality.
)

(event Collision|EventActorBeginOverlap
  (params (OtherActor :type Actor%20Object%20Reference))
  (|CallParentFunction OtherActor) ; This node is disabled and will not be called.\nDrag off pins to build functionality.
)

(event EventTick
  (params (DeltaSeconds :type Float%20%28single-precision%29))
  (|CallParentFunction DeltaSeconds) ; This node is disabled and will not be called.\nDrag off pins to build functionality.
)

(fn ConstructionScript
  (|CallParentFunction))

(fn AddSouls
  (params (Value :type Float%20%28double-precision%29))
  (Variables|Default|SetSouls (Math|Float|Max(Float) (Math|Float|Min(Float) (+ Value (Variables|Default|GetSouls)) (Variables|Default|GetMaxSouls)) 0.0)))

(fn FireSoul
  (params (HomingTarget :type Scene%20Component%20Object%20Reference) (DamageMult :type Float%20%28double-precision%29))
  (bind _returnvalue (Game|SpawnActorfromClass "/Game/BP_ShooterProjectile_Soul.BP_ShooterProjectile_Soul_C" (Math|Transform|MakeTransform (Transformation|GetActorLocation (Variables|Default|GetPawn%20Owner)) (Math|Random|RandomRotator false) "1.000000,1.000000,1.000000") "AlwaysSpawn" "MultiplyWithRoot" (Components|GetOwner) (Variables|Default|GetPawn%20Owner)))
  (Variables|/Game/Variant_Shooter/Blueprints/Pickups/Projectiles/BP_ShooterProjectileBase.BP_ShooterProjectileBase_C|SetDamage _returnvalue (* (Variables|Default|GetDamage) DamageMult))
  (Variables|/Game/BP_ShooterProjectile_Soul.BP_ShooterProjectile_Soul_C|SetTarget _returnvalue HomingTarget))

(fn GetNearestEnemy
  (params (Actor :type Actor%20Object%20Reference))
  (return (CallFunction|GetNearestEnemy Actor)))

(fn GetNearestEnemies
  (params (Actor :type Actor%20Object%20Reference))
  (return (CallFunction|GetNearestEnemies Actor)))

(fn FireBullet
  (params (Target%20Position :type Vector :default "0, 0, 0"))
  (|CallParentFunction Target%20Position)
  (CallFunction|AddSouls 1.0))

(fn OnRequiem
  (Variables|Default|SetCanGetSoul false)
  (Utilities|Time|SetTimerbyEvent (EventDispatchers|CreateEvent :!event ResetCanGetSoul) 1e+01))

(fn ResetCanGetSoul
  (Variables|Default|SetCanGetSoul true))