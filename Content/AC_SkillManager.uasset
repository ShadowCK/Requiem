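; Player skill manager component that creates, stores and triggers the soul-themed skills of its owning BP_Player.
; On BeginPlay it constructs seven skill objects bound to the player's caster component and registers each by name in a map at max level.
; Tick runs every skill's Passive update, while four input actions cast Soul Devour, Power Rite, Soul Imbalance and Requiem through name lookup.
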(event Input|EnhancedActionEvents|EnhancedInputActionIA_1
  (params (ActionValue :type Boolean) (ElapsedSeconds :type Float%20%28double-precision%29) (TriggeredSeconds :type Float%20%28double-precision%29) (InputAction :type Input%20Action%20Object%20Reference :default "/Game/IA_1.IA_1"))
  (:Started
    (CallFunction|CastSkillbyName "Soul Devour")))

(event Input|EnhancedActionEvents|EnhancedInputActionIA_2
  (params (ActionValue :type Boolean) (ElapsedSeconds :type Float%20%28double-precision%29) (TriggeredSeconds :type Float%20%28double-precision%29) (InputAction :type Input%20Action%20Object%20Reference :default "/Game/IA_2.IA_2"))
  (:Started
    (CallFunction|CastSkillbyName "Power Rite")))

(event Input|EnhancedActionEvents|EnhancedInputActionIA_3
  (params (ActionValue :type Boolean) (ElapsedSeconds :type Float%20%28double-precision%29) (TriggeredSeconds :type Float%20%28double-precision%29) (InputAction :type Input%20Action%20Object%20Reference :default "/Game/IA_3.IA_3"))
  (:Started
    (CallFunction|CastSkillbyName "Soul Imbalance")))

(event Input|EnhancedActionEvents|EnhancedInputActionIA_4
  (params (ActionValue :type Boolean) (ElapsedSeconds :type Float%20%28double-precision%29) (TriggeredSeconds :type Float%20%28double-precision%29) (InputAction :type Input%20Action%20Object%20Reference :default "/Game/IA_4.IA_4"))
  (:Started
    (CallFunction|CastSkillbyName "Requiem")))

(event EventBeginPlay
  (bind _asbp_player (Utilities|Casting|CastToBP_Player (Components|GetOwner)))
  (bind _output_get (Variables|Default|SetPlayer _asbp_player))
  (Variables|Default|SetCaster (Variables|/Game/BP_Player.BP_Player_C|GetAC_Caster _output_get))
  (bind _returnvalue (Game|ConstructObjectfromClass "/Game/Skills/SoulContainer.SoulContainer_C" (Variables|/Game/BP_Player.BP_Player_C|GetAC_Caster (Variables|Default|GetPlayer))))
  (bind _returnvalue_2 (Game|ConstructObjectfromClass "/Game/Skills/SoulDevour.SoulDevour_C" (Variables|/Game/BP_Player.BP_Player_C|GetAC_Caster (Variables|Default|GetPlayer))))
  (bind _returnvalue_3 (Game|ConstructObjectfromClass "/Game/Skills/SoulFurnace.SoulFurnace_C" (Variables|/Game/BP_Player.BP_Player_C|GetAC_Caster (Variables|Default|GetPlayer))))
  (bind _returnvalue_4 (Game|ConstructObjectfromClass "/Game/Skills/SoulHunger.SoulHunger_C" (Variables|/Game/BP_Player.BP_Player_C|GetAC_Caster (Variables|Default|GetPlayer))))
  (bind _returnvalue_5 (Game|ConstructObjectfromClass "/Game/Skills/SoulImbalance.SoulImbalance_C" (Variables|/Game/BP_Player.BP_Player_C|GetAC_Caster (Variables|Default|GetPlayer))))
  (bind _returnvalue_6 (Game|ConstructObjectfromClass "/Game/Skills/PowerRite.PowerRite_C" (Variables|/Game/BP_Player.BP_Player_C|GetAC_Caster (Variables|Default|GetPlayer))))
  (bind _returnvalue_7 (Game|ConstructObjectfromClass "/Game/Skills/Requiem.Requiem_C" (Variables|/Game/BP_Player.BP_Player_C|GetAC_Caster (Variables|Default|GetPlayer))))
  (CallFunction|AddSkill _returnvalue)
  (CallFunction|AddSkill _returnvalue_2)
  (CallFunction|AddSkill _returnvalue_3)
  (CallFunction|AddSkill _returnvalue_4)
  (CallFunction|AddSkill _returnvalue_5)
  (CallFunction|AddSkill _returnvalue_6)
  (CallFunction|AddSkill _returnvalue_7)
  (Development|PrintText "All skills added"))

(event EventTick
  (params (DeltaSeconds :type Float%20%28single-precision%29))
  (bind _valuepin (Utilities|Map|ForEachLoop(Map) (Variables|Default|GetSkills))
    (:then
      (Default|Passive _valuepin DeltaSeconds))))

(fn CastSkill
  (params (Skill :type BP%20Skill%20Base%20Object%20Reference))
  (Utilities|IsValid Skill
    (:Is%20Valid
      (Default|Cast Skill))))

(fn CastSkillbyName
  (params (SkillName :type String))
  (CallFunction|CastSkill (CallFunction|GetSkill SkillName)))

(fn GetSkill
  (params (SkillName :type String))
  (return (.Value (Utilities|Map|Find (Variables|Default|GetSkills) SkillName))))

(fn HasSkill
  (params (Name :type String))
  (return (.ReturnValue (Utilities|Map|Find (Variables|Default|GetSkills) Name))))

(fn AddSkill
  (params (Skill :type BP%20Skill%20Base%20Object%20Reference))
  (Utilities|Map|Add (Variables|Default|GetSkills) (Variables|/Game/Skills/BP_SkillBase.BP_SkillBase_C|GetName Skill) Skill)
  (Variables|/Game/Skills/BP_SkillBase.BP_SkillBase_C|SetLevel Skill (Variables|/Game/Skills/BP_SkillBase.BP_SkillBase_C|GetMaxLevel Skill)))